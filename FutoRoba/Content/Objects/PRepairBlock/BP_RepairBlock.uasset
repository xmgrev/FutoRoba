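; BP_RepairBlock is a world object that makes repair available to the player when the character reaches it.
; On BeginPlay it caches player controller 0 as PC_Game.
; When a BP_Char begins overlapping its Box, it stores itself as the controller's RepairBlockRef and sets CanRepair to true.
; It has no end-overlap handler, so it never clears either value itself.
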(event OnComponentBeginOverlap(Box)
  (params (OverlappedComponent :type Primitive%20Component%20Object%20Reference) (OtherActor :type Actor%20Object%20Reference) (OtherComp :type Primitive%20Component%20Object%20Reference) (OtherBodyIndex :type Integer) (bFromSweep :type Boolean) (SweepResult :type Hit%20Result%20Structure%20%28by%20ref%29))
  ;[0.1946 0.1946 0.1946] overlap
  (Utilities|Casting|CastToBP_Char OtherActor)
  (Variables|/Game/Core/PC_Game.PC_Game_C|SetRepairBlockRef (Variables|Default|GetPC) self)
  (Variables|/Game/Core/PC_Game.PC_Game_C|SetcanRepair (Variables|Default|GetPC) true))

(event Custom|refereces
  ;[0.1946 0.1946 0.1946] references
  (bind _aspc_game (Utilities|Casting|CastToPC_Game (Game|GetPlayerController 0)))
  (Variables|Default|SetPC _aspc_game))

(event EventBeginPlay
  ;[0.1946 0.1946 0.1946] initchain
  (CallFunction|Refereces))

(fn ConstructionScript)