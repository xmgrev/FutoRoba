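; BP_C_collider is a one-shot trigger volume that advances the level's camera and boundaries when the player character overlaps its box.
; It caches the PC_Game controller on BeginPlay, then on overlap teleports that controller's player blocker, camera and dead zone to fixed offsets from its own location.
; The blocker lands behind along X, the camera above and the dead zone below, after which the collider destroys itself.
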(event OnComponentBeginOverlap(Box)
  (params (OverlappedComponent :type Primitive%20Component%20Object%20Reference) (OtherActor :type Actor%20Object%20Reference) (OtherComp :type Primitive%20Component%20Object%20Reference) (OtherBodyIndex :type Integer) (bFromSweep :type Boolean) (SweepResult :type Hit%20Result%20Structure%20%28by%20ref%29))
  ;[0.1946 0.1946 0.1946] overlap
  (Utilities|Casting|CastToBP_Char OtherActor)
  (CallFunction|MovePlayerBlock)
  (CallFunction|MoveCamera)
  (CallFunction|MoveDeadZone)
  (Actor|DestroyActor))

(event Custom|references
  ;[0.1946 0.1946 0.1946] Comment
  (bind _aspc_game (Utilities|Casting|CastToPC_Game (Game|GetPlayerController 0)))
  (Variables|Default|SetPC _aspc_game))

(event Custom|MovePlayerBlock
  ;[0.1946 0.1946 0.1946] MovePlayerBlock
  (Transformation|SetActorLocation (Variables|/Game/Core/PC_Game.PC_Game_C|GetBlockPlayer (Variables|Default|GetPC)) (- (Transformation|GetActorLocation) "1100.000000,0.000000,0.000000") false true))

(event Custom|MoveCamera
  ;[0.1946 0.1946 0.1946] Move camera
  (Transformation|SetActorLocation (Variables|/Game/Core/PC_Game.PC_Game_C|GetCameraRef (Variables|Default|GetPC)) (+ (Transformation|GetActorLocation) "0.000000,0.000000,250.000000") false true))

(event Custom|MoveDeadZone
  ;[0.1946 0.1946 0.1946] move dead zone
  (Transformation|SetActorLocation (Variables|/Game/Core/PC_Game.PC_Game_C|GetDeadZone (Variables|Default|GetPC)) (- (Transformation|GetActorLocation) "0.000000,0.000000,400.000000") false true))

(event EventBeginPlay
  ;[0.1946 0.1946 0.1946] initchain
  (CallFunction|References))

(fn ConstructionScript)